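; BP_PlayerCharacter is a player character Blueprint that shows its health on a widget-based health bar.
; BeginPlay gets the BP_HealthBar widget from HealthBarWidget, creates a dynamic material from its image, stores the starting health and sets the Percentage parameter.
; Tick sets that parameter from current health, normalized to 100, whenever health is below the stored starting value, which is never updated afterward.
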(event EventBeginPlay
  (bind _returnvalue (Class|BaseCharacter|GetHealth))
  (bind _asbp_health_bar (Utilities|Casting|CastToBP_HealthBar (UserInterface|GetUserWidgetObject (Variables|Default|GetHealthBarWidget))))
  (bind _output_get (Variables|Default|SetHealthBar _asbp_health_bar))
  (bind _returnvalue_2 (Appearance|GetDynamicMaterial (Variables|/Game/Blueprints/BP_HealthBar.BP_HealthBar_C|GetImage_0 _output_get) :!class /Script/UMG.Image))
  (bind _output_get_2 (Variables|Default|SetHealthBarMaterial _returnvalue_2))
  (Variables|Default|SetPlayerHealth _returnvalue)
  (Rendering|Material|SetScalarParameterValue _output_get_2 "Percentage" (/ _returnvalue 1e+02) :!class /Script/Engine.MaterialInstanceDynamic))

(event EventTick
  (params (DeltaSeconds :type Float%20%28single-precision%29))
  (bind _returnvalue (Class|BaseCharacter|GetHealth))
  (if (< _returnvalue (Variables|Default|GetPlayerHealth))
    (Rendering|Material|SetScalarParameterValue (Variables|Default|GetHealthBarMaterial) "Percentage" (/ _returnvalue 1e+02) :!class /Script/Engine.MaterialInstanceDynamic)))

(fn ConstructionScript)