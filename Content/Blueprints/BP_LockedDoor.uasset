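; Locked-capable door that slides between a raised start position and its placed position when a valid character overlaps it.
; BeginPlay raises the door and, if it is locked, spawns a key-carrying enemy at a fixed world offset, passing it a reference to the door.
; Overlaps with BaseCharacters that pass IsTriggeringCharacterValid play the DoorOpening timeline, lerping the door down; end overlap reverses it.
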(event Collision|EventActorBeginOverlap
  (params (OtherActor :type Actor%20Object%20Reference))
  ;[1 1 1] Open/close door when appropriate actor overlaps/leaves trigger zone.
  (bind _asbase_character (Utilities|Casting|CastToBaseCharacter OtherActor))
  (bind _returnvalue (Class|LockedDoor|IsTriggeringCharacterValid _asbase_character))
  (if _returnvalue
    (bind _door_track (Timeline|DoorOpening Play)
      (:Update
        (Transformation|SetActorLocation (Math|Vector|Lerp(Vector) (Variables|Default|GetStartingLocation) (Variables|Default|GetEndingLocation) _door_track) false false)))))

(event EventBeginPlay
  (bind _returnvalue (Transformation|GetActorLocation))
  ;[1 1 1] Setup Doors.
  (bind _output_get (Variables|Default|SetStartingLocation (+ "0, 0,235.000000" _returnvalue)))
  (Variables|Default|SetEndingLocation _returnvalue)
  (Transformation|SetActorLocation _output_get false false)
  (bind _returnvalue_2 (Class|LockedDoor|GetIsLocked))
  (if _returnvalue_2
    (bind _returnvalue_3 (Game|SpawnActorfromClass "/Game/Blueprints/Characters/BP_EnemyKeyCharacter.BP_EnemyKeyCharacter_C" (Math|Transform|MakeTransform (+ (Math|Transform|TransformLocation (Transformation|GetActorTransform) "0, 0, 0") "0,1500.000000, 0")) "Undefined" 0 0))
    (Variables|/Script/Sleuth.EnemyKeyCharacter|SetLockedDoor _returnvalue_3 self)))

(event Collision|EventActorEndOverlap
  (params (OtherActor :type Actor%20Object%20Reference))
  ;[1 1 1] Open/close door when appropriate actor overlaps/leaves trigger zone.
  (bind _asbase_character (Utilities|Casting|CastToBaseCharacter OtherActor))
  (bind _returnvalue (Class|LockedDoor|IsTriggeringCharacterValid _asbase_character))
  (if _returnvalue
    (bind _door_track (Timeline|DoorOpening Reverse)
      (:Update
        (Transformation|SetActorLocation (Math|Vector|Lerp(Vector) (Variables|Default|GetStartingLocation) (Variables|Default|GetEndingLocation) _door_track) false false)))))

(fn ConstructionScript)